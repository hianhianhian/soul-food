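; Player controller for a dialogue game that locks look and move input and focuses game-and-UI input on the game mode's HUD widget.
; GameStarted sets a flag and switches the placeholder flipbook handler to the background flipbook.
; Once started, Interact messages the menu controller found at BeginPlay through BPI_Interact.
; Directional select inputs and the click handler only print debug text; the cafe camera view-target logic is unconnected.
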(event Custom|GameStarted
  (Variables|Default|SetGameStarted? true)
  (bind _outactors (Actor|GetAllActorsOfClass "/Game/Blueprints/BP_PlaceholderFlipbookHandler.BP_PlaceholderFlipbookHandler_C"))
  (Sprite|SetFlipbook (Variables|/Script/Paper2D.PaperFlipbookActor|GetRenderComponent (Utilities|Array|Get(acopy) _outactors)) "/Game/Assets/FB_background.FB_background"))

(event Custom|OnClicked_Event_0
  (params (TouchedActor :type Actor%20Object%20Reference) (ButtonPressed :type Key%20Structure))
  (Development|PrintString "Hello"))

(event EventBeginPlay
  (Utilities|FlowControl|Sequence
    (:then_0
      (Input|SetIgnoreLookInput true)
      (Input|SetIgnoreMoveInput true))
    (:then_1
      (bind _asbp_dialogue_game_mode (Utilities|Casting|CastToBP_DialogueGameMode (Game|GetGameMode)))
      (bind _output_get (Variables|Default|SetPlayerHUDRef (Variables|/Game/Blueprints/BP_DialogueGameMode.BP_DialogueGameMode_C|GetHeadsUpDisplay _asbp_dialogue_game_mode)))
      (Input|SetInputModeGameandUI self _output_get "LockOnCapture" false))
    (:then_2
      (bind _outactors (Actor|GetAllActorsOfClass "/Game/Blueprints/BP_MenuController.BP_MenuController_C"))
      (Variables|Default|SetAI_MenuControllerRef (Utilities|Array|Get(acopy) _outactors))
      (EventDispatchers|AssignOnClicked (delegate Custom|OnClicked_Event_0)))))

(event Input|ActionEvents|InputActionSelectAbove
  (params (Key :type Key%20Structure))
  (:Pressed
    (Development|PrintString (Utilities|String|ToString(Text) (Class|KismetInputLibrary|KeyGetDisplayName Key)))))

(event Input|ActionEvents|InputActionSelectBelow
  (params (Key :type Key%20Structure))
  (:Pressed
    (Development|PrintString (Utilities|String|ToString(Text) (Class|KismetInputLibrary|KeyGetDisplayName Key)))))

(event Input|ActionEvents|InputActionSelectLeft
  (params (Key :type Key%20Structure))
  (:Pressed
    (Development|PrintString (Utilities|String|ToString(Text) (Class|KismetInputLibrary|KeyGetDisplayName Key)))))

(event Input|ActionEvents|InputActionSelectRight
  (params (Key :type Key%20Structure))
  (:Pressed
    (Development|PrintString (Utilities|String|ToString(Text) (Class|KismetInputLibrary|KeyGetDisplayName Key)))))

(event Input|ActionEvents|InputActionInteract
  (params (Key :type Key%20Structure))
  (bind _ai_menucontrollerref (Variables|Default|GetAI_MenuControllerRef))
  (:Pressed
    (Development|PrintString (Utilities|String|ToString(Text) (Class|KismetInputLibrary|KeyGetDisplayName Key)))
    (if (and (Variables|Default|GetGameStarted?) (Utilities|DoesObjectImplementInterface _ai_menucontrollerref "/Game/Blueprints/BPI_Interact.BPI_Interact_C"))
      (Class|BPIInteract|Interact(Message) _ai_menucontrollerref))))

(fn ConstructionScript)