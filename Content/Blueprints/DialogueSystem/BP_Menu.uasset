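; Menu handler owned by BP_MenuController that displays a selectable dish menu and the serve button for the chosen dish.
; ShowMenu rebuilds the menu widget in the game mode's HUD overlay, with one item per non-empty entry.
; A clicked item passes its ingredient branch to the controller, then rebuilds the dish button from the matching DT_Menu row.
; Button opacity tracks collected versus required ingredients, enabling serving when complete.
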(event Custom|ShowMenu
  (params (MenuItems :type Array%20of%20S%20Menu%20Data%20Structures))
  (Variables|Default|SetMenuList MenuItems)
  (bind _asbp_dialogue_game_mode (Utilities|Casting|CastToBP_DialogueGameMode (Game|GetGameMode)))
  (Variables|Default|SetHUDRef (Variables|/Game/Blueprints/BP_DialogueGameMode.BP_DialogueGameMode_C|GetHeadsUpDisplay _asbp_dialogue_game_mode))
  (Utilities|IsValid (Variables|Default|GetMenuWidgetRef)
    (:Is%20Valid
      (Widget|SetVisibility (Variables|Default|GetMenuWidgetRef) "Collapsed")
      (Widget|Panel|ClearChildren (Variables|/Game/Widgets/BPWidget_Menu.BPWidget_Menu_C|GetSizeBox_27 (Variables|Default|GetMenuWidgetRef)))
      (Widget|RemovefromParent (Variables|Default|GetMenuWidgetRef))
      (Variables|Default|SetMenuWidgetRef (Variables|Default|GetNULLMenuWidgetRef))
      (CallFunction|PrepareMenuList))
    (:Is%20Not%20Valid
      (CallFunction|PrepareMenuList))))

(event Custom|MenuItemReceived
  (params (Response :type Name))
  (Default|IngredientsBranchReceived (Variables|Default|GetMenuControllerRef) Response)
  ;[1 1 1] Check validity/generate a new dish button widget
  (Utilities|IsValid (Variables|Default|GetDishButtonRef)
    (:Is%20Valid
      (Widget|SetVisibility (Variables|Default|GetDishButtonRef) "Collapsed")
      (Widget|Panel|ClearChildren (Variables|/Game/Widgets/BPWidget_DishButton.BPWidget_DishButton_C|GetSizeBox_35 (Variables|Default|GetDishButtonRef)))
      (Widget|RemovefromParent (Variables|Default|GetDishButtonRef))
      (Variables|Default|SetDishButtonRef 0)
      (CallFunction|PrepareDishButton Response))
    (:Is%20Not%20Valid
      (CallFunction|PrepareDishButton Response))))

(event EventBeginPlay
  (EventDispatchers|BindEventtoMenuItemClicked (delegate Custom|MenuItemReceived))
  (bind _asbp_menu_controller (Utilities|Casting|CastToBP_MenuController (Components|GetOwner)))
  (Variables|Default|SetMenuControllerRef _asbp_menu_controller))

(event EventTick
  (params (DeltaSeconds :type Float%20%28single-precision%29)))

(fn PrepareMenuList
  (bind _returnvalue (UserInterface|CreateWidget "/Game/Widgets/BPWidget_Menu.BPWidget_Menu_C"))
  (bind _output_get (Variables|Default|SetMenuWidgetRef _returnvalue))
  (bind _returnvalue_2 (Class|Overlay|AddChildtoOverlay (Variables|/Game/Widgets/BPWidget_HUD.BPWidget_HUD_C|GetMenuOverlay (Variables|Default|GetHUDRef)) _output_get))
  (Layout|GridSlot|SetHorizontalAlignment _returnvalue_2 "HAlign_Center")
  (Layout|GridSlot|SetVerticalAlignment _returnvalue_2 "VAlign_Center")
  (Layout|BorderSlot|SetPadding :self _returnvalue_2 :!class /Script/UMG.OverlaySlot)
  (for _array_element (Variables|Default|GetMenuList)
    (if (not (Utilities|Text|TextIsEmpty (.Text (Utilities|Struct|BreakS_MenuData _array_element))))
      (bind _returnvalue_3 (UserInterface|CreateWidget "/Game/Widgets/BPWidget_MenuItem.BPWidget_MenuItem_C" 0 self _array_element))
      (Class|VerticalBox|AddChildtoVerticalBox (Variables|/Game/Widgets/BPWidget_Menu.BPWidget_Menu_C|GetMenuList (Variables|Default|GetMenuWidgetRef)) _returnvalue_3))))

(fn PrepareDishButton
  (params (IngredientBranch :type Name))
  (bind _outrownames (DataTable|GetDataTableRowNames "/Game/Data/DT_Menu.DT_Menu"))
  (for _array_element _outrownames
    (bind _returnvalue (Utilities|GetDataTableRow "/Game/Data/DT_Menu.DT_Menu" _array_element)
      (:then
        (if (Utilities|Name|Equal(Name) (.IngredientsBranch (Utilities|Struct|BreakS_MenuData _returnvalue)) IngredientBranch)
          (bind _returnvalue_2 (UserInterface|CreateWidget "/Game/Widgets/BPWidget_DishButton.BPWidget_DishButton_C" 0 (Utilities|String|StringToName (Utilities|String|BuildString(Name) "" "" (.IngredientsBranch (Utilities|Struct|BreakS_MenuData _returnvalue)) ":5")) (.DishIcon (Utilities|Struct|BreakS_MenuData _returnvalue))))
          (bind _output_get (Variables|Default|SetDishButtonRef _returnvalue_2))
          (CallFunction|SetDishButtonOpacity)
          (Class|Overlay|AddChildtoOverlay (Variables|/Game/Widgets/BPWidget_HUD.BPWidget_HUD_C|GetDishPortraitOverlay (Variables|Default|GetHUDRef)) _output_get))))))

(fn SetDishButtonOpacity
  (bind _dishbuttonref (Variables|Default|GetDishButtonRef))
  (bind _menucontrollerref (Variables|Default|GetMenuControllerRef))
  (bind _innerborder (Variables|/Game/Widgets/BPWidget_DishButton.BPWidget_DishButton_C|GetInnerBorder _dishbuttonref))
  (Widget|SetRenderOpacity _innerborder (/ (Math|Conversions|ToFloat(Integer) (Variables|/Game/Blueprints/BP_MenuController.BP_MenuController_C|GetCurrentTotalIngredientCounter _menucontrollerref)) (Math|Conversions|ToFloat(Integer) (Variables|/Game/Blueprints/BP_MenuController.BP_MenuController_C|GetCurrentMenuRequiredNum _menucontrollerref))))
  (if (>= (Class|Widget|GetRenderOpacity _innerborder) 1.0)
    (Widget|SetIsEnabled (Variables|/Game/Widgets/BPWidget_DishButton.BPWidget_DishButton_C|GetDishServeButton _dishbuttonref) true)
    (Class|Border|SetBrushColor (Variables|/Game/Widgets/BPWidget_DishButton.BPWidget_DishButton_C|GetOuterBorder _dishbuttonref) "(R=1.000000,G=1.000000,B=1.000000,A=0.420000)")))

(fn ClearMenuBorders
  (for _array_element (Class|PanelWidget|GetAllChildren (Variables|/Game/Widgets/BPWidget_Menu.BPWidget_Menu_C|GetMenuList (Variables|Default|GetMenuWidgetRef)))
    (bind _asbpwidget_menu_item (Utilities|Casting|CastToBPWidget_MenuItem _array_element))
    (Class|Border|SetBrushColor (Variables|/Game/Widgets/BPWidget_MenuItem.BPWidget_MenuItem_C|GetOuterBorder _asbpwidget_menu_item) "(R=0.093059,G=0.093059,B=0.093059,A=0.000000)")))