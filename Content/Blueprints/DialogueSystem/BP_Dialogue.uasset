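; BP_Dialogue displays one dialogue text at a time in a box on the HUD.
; ShowDialogue stores the text and final-branch flag, gets the HUD from BP_DialogueGameMode, and tears down any existing dialogue widget.
; PrepareDialogueBox then creates a fresh BPWidget_DialogueBox in the HUD's DialogueOverlay, showing the click cursor and screen-click button only on non-final branches.
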(event Custom|ShowDialogue
  (params (Text :type Text) (isFinalBranch :type Boolean))
  (Variables|Default|SetDialogueText Text)
  (Variables|Default|SetisFinalBranch isFinalBranch)
  (bind _asbp_dialogue_game_mode (Utilities|Casting|CastToBP_DialogueGameMode (Game|GetGameMode)))
  (Variables|Default|SetHUDRef (Variables|/Game/Blueprints/BP_DialogueGameMode.BP_DialogueGameMode_C|GetHeadsUpDisplay _asbp_dialogue_game_mode))
  (Utilities|IsValid (Variables|Default|GetDialogueWidgetRef)
    (:Is%20Valid
      (Widget|SetVisibility (Variables|Default|GetDialogueWidgetRef) "Collapsed")
      (Widget|Panel|ClearChildren (Variables|/Game/Widgets/BPWidget_DialogueBox.BPWidget_DialogueBox_C|GetSizeBox_40 (Variables|Default|GetDialogueWidgetRef)))
      (Widget|RemovefromParent (Variables|Default|GetDialogueWidgetRef))
      (Variables|Default|SetDialogueWidgetRef (Variables|Default|GetNULLDialogueWidgetRef))
      (CallFunction|PrepareDialogueBox))
    (:Is%20Not%20Valid
      (CallFunction|PrepareDialogueBox))))

(event EventBeginPlay)

(fn PrepareDialogueBox
  (bind _hudref (Variables|Default|GetHUDRef))
  (bind _screenclickbutton (Variables|/Game/Widgets/BPWidget_HUD.BPWidget_HUD_C|GetScreenClickButton _hudref))
  (bind _returnvalue (UserInterface|CreateWidget "/Game/Widgets/BPWidget_DialogueBox.BPWidget_DialogueBox_C" 0 (Variables|Default|GetDialogueText)))
  (bind _output_get (Variables|Default|SetDialogueWidgetRef _returnvalue))
  (Class|Overlay|AddChildtoOverlay (Variables|/Game/Widgets/BPWidget_HUD.BPWidget_HUD_C|GetDialogueOverlay _hudref) _output_get)
  (if (Variables|Default|GetisFinalBranch)
    (Widget|SetVisibility (Variables|/Game/Widgets/BPWidget_DialogueBox.BPWidget_DialogueBox_C|GetCursorClickImage _output_get) "Hidden")
    (Widget|SetVisibility _screenclickbutton "Collapsed")
    (else
      (Widget|SetVisibility (Variables|/Game/Widgets/BPWidget_DialogueBox.BPWidget_DialogueBox_C|GetCursorClickImage _output_get) "Visible")
      (Widget|SetVisibility _screenclickbutton "Visible"))))