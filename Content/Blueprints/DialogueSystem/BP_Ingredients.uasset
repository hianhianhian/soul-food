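; Menu controller component that shows a clickable ingredient list in the dialogue HUD and forwards the chosen response to the controller as a dialogue branch.
; ShowIngredientsList rebuilds the widget, placing items in a two-by-two grid with usage counters from the controller.
; IDs ending in "5" or "Final" are skipped.
; A Love button spans a third column, its "Final" ID derived by trimming the last key's name.
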(event Custom|ShowIngredientsList
  (params (IngredientsList :type Map%20of%20Names%20to%20Structs))
  (Variables|Default|SetIngredientsList IngredientsList)
  (bind _asbp_dialogue_game_mode (Utilities|Casting|CastToBP_DialogueGameMode (Game|GetGameMode)))
  (Variables|Default|SetHUDRef (Variables|/Game/Blueprints/BP_DialogueGameMode.BP_DialogueGameMode_C|GetHeadsUpDisplay _asbp_dialogue_game_mode))
  (Utilities|IsValid (Variables|Default|GetIngredientsListWidgetRef)
    (:Is%20Valid
      (Widget|SetVisibility (Variables|Default|GetIngredientsListWidgetRef) "Collapsed")
      (Widget|Panel|ClearChildren (Variables|/Game/Widgets/BPWidget_IngredientsList.BPWidget_IngredientsList_C|GetSizeBox_44 (Variables|Default|GetIngredientsListWidgetRef)))
      (Widget|RemovefromParent (Variables|Default|GetIngredientsListWidgetRef))
      (Variables|Default|SetIngredientsListWidgetRef (Variables|Default|GetNULLIngredientsListWidgetRef))
      (CallFunction|PrepareIngredientsList))
    (:Is%20Not%20Valid
      (CallFunction|PrepareIngredientsList))))

(event Custom|IngredientResponseReceived
  (params (Response :type Name))
  (Default|DialogueBranchReceived (Variables|Default|GetOwnerRef) Response))

(event EventTick
  (params (DeltaSeconds :type Float%20%28single-precision%29)))

(event EventBeginPlay
  (EventDispatchers|BindEventtoIngredientItemClicked (delegate Custom|IngredientResponseReceived))
  (bind _asbp_menu_controller (Utilities|Casting|CastToBP_MenuController (Components|GetOwner)))
  (Variables|Default|SetOwnerRef _asbp_menu_controller))

(fn PrepareIngredientsList
  (bind _returnvalue (UserInterface|CreateWidget "/Game/Widgets/BPWidget_IngredientsList.BPWidget_IngredientsList_C"))
  (bind _output_get (Variables|Default|SetIngredientsListWidgetRef _returnvalue))
  (Class|Overlay|AddChildtoOverlay (Variables|/Game/Widgets/BPWidget_HUD.BPWidget_HUD_C|GetIngredientOverlay (Variables|Default|GetHUDRef)) _output_get)
  (bind _keys (Utilities|Map|Keys (Variables|Default|GetIngredientsList)))
  (for (_array_element _array_index) _keys
    (bind _output_get_2 (Variables|Default|SetcurrentID _array_element))
    (if (and (not (Utilities|String|EndsWith (Utilities|String|ToString(Name) _output_get_2) "5")) (not (Utilities|String|EndsWith (Utilities|String|ToString(Name) _output_get_2) "Final")))
      (bind (_ingredientsdata _ingredientcounter) (CallFunction|ExtractData (Variables|Default|GetIngredientsList) (Variables|Default|GetcurrentID)))
      (bind _returnvalue_2 (UserInterface|CreateWidget "/Game/Widgets/BPWidget_IngredientItem.BPWidget_IngredientItem_C" 0 (Variables|Default|GetcurrentID) _ingredientsdata self _ingredientcounter))
      (bind _output_get_3 (Variables|Default|SetIngredientItemRef _returnvalue_2))
      (bind _returnvalue_3 (Class|GridPanel|AddChildtoGrid (Variables|/Game/Widgets/BPWidget_IngredientsList.BPWidget_IngredientsList_C|GetIngredientsList (Variables|Default|GetIngredientsListWidgetRef)) _output_get_3))
      (Class|GridSlot|SetRow _returnvalue_3 (Math|Float|Round (.X (Math|Vector2D|BreakVector2D (Utilities|Select :Index _array_index :Option%200 (LocalVariables|GetRow0Column0) :Option%201 (LocalVariables|GetRow0Column1) :Option%202 (LocalVariables|GetRow1Column0) :Option%203 (LocalVariables|GetRow1Column1))))))
      (Class|GridSlot|SetColumn _returnvalue_3 (Math|Float|Round (.Y (Math|Vector2D|BreakVector2D (Utilities|Select :Index _array_index :Option%200 (LocalVariables|GetRow0Column0) :Option%201 (LocalVariables|GetRow0Column1) :Option%202 (LocalVariables|GetRow1Column0) :Option%203 (LocalVariables|GetRow1Column1))))))
      (Layout|BorderSlot|SetPadding _returnvalue_3 (Utilities|Struct|MakeMargin 4.0 4.0 4.0 4.0) :!class /Script/UMG.GridSlot)))
  (bind _returnvalue_4 (UserInterface|CreateWidget "/Game/Widgets/BPWidget_LoveButton.BPWidget_LoveButton_C" 0 (Utilities|String|StringToName (Utilities|String|Append (Utilities|String|LeftChop (Utilities|String|ToString(Name) (Variables|Default|GetcurrentID)) 3) "Final")) self))
  (bind _output_get_4 (Variables|Default|SetLoveButtonRef _returnvalue_4))
  (bind _returnvalue_5 (Class|GridPanel|AddChildtoGrid (Variables|/Game/Widgets/BPWidget_IngredientsList.BPWidget_IngredientsList_C|GetIngredientsList (Variables|Default|GetIngredientsListWidgetRef)) _output_get_4))
  (Class|GridSlot|SetRow _returnvalue_5)
  (Class|GridSlot|SetRowSpan _returnvalue_5 2)
  (Class|GridSlot|SetColumn _returnvalue_5 2)
  (Layout|BorderSlot|SetPadding _returnvalue_5 (Utilities|Struct|MakeMargin 6.0 6.0 6.0 6.0) :!class /Script/UMG.GridSlot))

(fn ExtractData
  (params (IngredientsList :type Map%20of%20Names%20to%20Structs) (Key :type Name%20%28by%20ref%29))
  (bind (_value _returnvalue) (Utilities|Map|Find IngredientsList Key))
  (bind _ownerref (Variables|Default|GetOwnerRef))
  (bind _ingredientscounter (Variables|/Game/Blueprints/BP_MenuController.BP_MenuController_C|GetIngredientsCounter _ownerref))
  (bind (_value_2 _returnvalue_2) (Utilities|Map|Find _ingredientscounter Key))
  (if _returnvalue
    (if _returnvalue_2
      (LocalVariables|SetReturnCounter _value_2)
      (else
        (LocalVariables|SetReturnCounter 0)))
    (return _value (LocalVariables|GetReturnCounter))))